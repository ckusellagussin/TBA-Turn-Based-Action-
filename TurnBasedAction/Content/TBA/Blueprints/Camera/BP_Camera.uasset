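; Camera Blueprint that spawns the main hero at its own location on BeginPlay and follows it.
; BeginPlay also adds the camera Enhanced Input mapping context for player 0, stores the hero reference and shows the mouse cursor.
; The zoom input action feeds ZoomIn, which, like FollowTarget, is called rather than implemented here.
; An EnableFeatures call is left unconnected and never runs.
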(event `self.ReceiveBeginPlay`
  (`|ExecutionSequence`
    (:`then_0`
      (`EnhancedInputSubsystemInterface.AddMappingContext` (pcsubsystem `EnhancedInputLocalPlayerSubsystem` (`GameplayStatics.GetPlayerController` 0)) "/Game/TBA/Input/IMA_Camera.IMA_Camera" 0 (struct))
      (bind _returnvalue (`|SpawnActorFromClass` "/Game/TBA/Blueprints/Character/BP_MainHero.BP_MainHero_C" (`KismetMathLibrary.MakeTransform` (`self.K2_GetActorLocation`)) "Undefined" "MultiplyWithRoot" null self))
      (bind _output_get (set `self.BP_Hero` _returnvalue))
      (`self.FollowTarget` (`self.UseActor` _output_get)))
    (:`then_1`
      (set `PlayerController.bShowMouseCursor` true (`GameplayStatics.GetPlayerController` 0)))))

(event `EnhancedInput|/Game/TBA/Input/IA_CameraZoom`
  (params (ActionValue :type "Float (double-precision)") (ElapsedSeconds :type "Float (double-precision)") (TriggeredSeconds :type "Float (double-precision)") (InputAction :type "InputAction Object Reference" :default "/Game/TBA/Input/IA_CameraZoom.IA_CameraZoom"))
  (:`Triggered`
    (`self.ZoomIn` ActionValue)))

(fn `UserConstructionScript`)